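; Player pawn with camera-relative movement, sprinting, a coin count and a scroll goal.
; A looping timer drops a coin whenever flat speed reaches sprint speed, spawning a physics pickup launched in a random direction.
; First damage kills the player, triggering ragdoll, a full coin spill, effects and music through PNGameMode.
; ObtainScroll freezes movement, sets the scroll flag and switches music; the C key is a coin cheat.
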(event Custom|ObtainScroll
  ;[1 1 1] 巻物を入手
  (Utilities|FlowControl|Sequence
    (:then_0
      (Pawn|Components|CharacterMovement|DisableMovement (Variables|Character|GetCharacterMovement))
      (Variables|Default|SetHasScroll true)
      (Utilities|FlowControl|Delay 5.0)
      (Development|PrintString "Goal!"))
    (:then_1
      (Utilities|FlowControl|Delay 1.0)
      (Default|PlayBGM (.AsPNGame%20Mode (Utilities|Casting|CastToPNGameMode (Game|GetGameMode))) "/Game/Audio/bgm04_Cue.bgm04_Cue"))))

(event Custom|DropAllCoins
  ;[1 1 1] 死亡処理
  (while (> (Variables|Default|GetNumOfCoins) 0)
    (CallFunction|DropCoin)))

(event EventBeginPlay
  (Variables|/Script/Engine.CharacterMovementComponent|SetMaxWalkSpeed (Variables|Character|GetCharacterMovement) (Variables|キャラクター|GetGroundWalkSpeed))
  (Utilities|Time|SetTimerbyFunctionName 0 "CheckSprintRisk" 0.5 true))

(event Game|Damage|EventAnyDamage
  (params (Damage :type Float%20%28single-precision%29) (DamageType :type Damage%20Type%20Object%20Reference) (InstigatedBy :type Controller%20Object%20Reference) (DamageCauser :type Actor%20Object%20Reference))
  ;[1 1 1] 死亡処理
  (Utilities|FlowControl|DoOnce false
    (:Completed
      (Utilities|FlowControl|Sequence
        (:then_0
          (Development|PrintString "Died!")
          (Pawn|Components|CharacterMovement|DisableMovement (Variables|Character|GetCharacterMovement))
          (Actor|SetLifeSpan 5.0)
          (Collision|SetCollisionProfileName (Variables|Character|GetMesh) "Ragdoll" true :!class /Script/Engine.PrimitiveComponent)
          (Collision|SetCollisionProfileName (Variables|Collision|GetCapsuleComponent) "Spectator" true :!class /Script/Engine.PrimitiveComponent)
          (Physics|SetSimulatePhysics (Variables|Character|GetMesh) true))
        (:then_1
          (CallFunction|DropAllCoins))
        (:then_2
          (Components|Activation|Activate (Variables|Default|GetDeathFX) true)
          (Audio|PlaySoundatLocation "/Game/Audio/player_death_Cue.player_death_Cue" (Transformation|GetActorLocation) "0, 0, 0" 1.0 1.0 0.0 0 0 0)
          (Utilities|FlowControl|Delay 1.0)
          (Default|PlayBGM (.AsPNGame%20Mode (Utilities|Casting|CastToPNGameMode (Game|GetGameMode))) "/Game/Audio/bgm03_Cue.bgm03_Cue"))))))

(event Input|ActionEvents|InputActionSprint
  (params (Key :type Key%20Structure :default "None"))
  (bind _charactermovement (Variables|Character|GetCharacterMovement))
  ;[1 1 1] 移動
  (:Pressed
    (Variables|/Script/Engine.CharacterMovementComponent|SetMaxWalkSpeed _charactermovement (Variables|Character|GetGroundSprintSpeed)))
  (:Released
    (Variables|/Script/Engine.CharacterMovementComponent|SetMaxWalkSpeed _charactermovement (Variables|キャラクター|GetGroundWalkSpeed))))

(event Input|AxisEvents|InputAxisMoveForward
  (params (AxisValue :type Float%20%28single-precision%29))
  ;[1 1 1] 移動
  (Pawn|Input|AddMovementInput (CallFunction|FlattenDirection (Math|Vector|GetForwardVector (Variables|Default|GetCamera))) AxisValue false) ; 前進
)

(event Input|AxisEvents|InputAxisMoveRight
  (params (AxisValue :type Float%20%28single-precision%29))
  ;[1 1 1] 移動
  (Pawn|Input|AddMovementInput (CallFunction|FlattenDirection (Math|Vector|GetRightVector (Variables|Default|GetCamera))) AxisValue false))

(event Input|AxisEvents|InputAxisLookUp
  (params (AxisValue :type Float%20%28single-precision%29))
  ;[1 1 1] 見回し
  (Pawn|Input|AddControllerPitchInput AxisValue))

(event Input|AxisEvents|InputAxisLookRight
  (params (AxisValue :type Float%20%28single-precision%29))
  ;[1 1 1] 見回し
  (Pawn|Input|AddControllerYawInput AxisValue))

(event Input|KeyboardEvents|C
  (params (Key :type Key%20Structure :default "None"))
  ;[1 1 1] チート
  (:Pressed
    (CallFunction|AddCoin 1)))

(fn ConstructionScript)

(fn AddCoin
  (params (Num :type Integer))
  (Variables|Default|SetNumOfCoins (+ (Variables|Default|GetNumOfCoins) Num)))

(fn GetNumOfCoins
  (return (Variables|Default|GetNumOfCoins)))

(fn DropCoin
  (Math|Integer|CompareInt (Variables|Default|GetNumOfCoins) 1
    (:>
      _)
    (:==
      _))
  (Variables|Default|SetNumOfCoins (- (Variables|Default|GetNumOfCoins) 1))
  (bind _returnvalue (Game|SpawnActorfromClass "/Game/Blueprints/PNPickupCoinActor.PNPickupCoinActor_C" (Transformation|GetSocketTransform (Variables|Character|GetMesh) "CoinSpawnPoint" "RTS_World") "Undefined" 0 0))
  (Physics|SetSimulatePhysics (Variables|/Script/Engine.StaticMeshActor|GetStaticMeshComponent _returnvalue) true)
  (Physics|AddImpulse (Variables|/Script/Engine.StaticMeshActor|GetStaticMeshComponent _returnvalue) (Math|Vector|RotateVectorAroundAxis (Math|Vector|MakeVector 2e+02 0.0 2e+02) (Math|Random|RandomFloatinRange 0.0 3.6e+02) "0, 0,1.000000") "None" true))

(fn CheckSprintRisk
  (if (>= (Utilities|GetFlatSpeed) (Variables|Character|GetGroundSprintSpeed))
    (CallFunction|DropCoin)))