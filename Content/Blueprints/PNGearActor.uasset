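; PNGearActor is a gear actor that spins continuously around its yaw axis.
; The construction script uses a shared DestroyGear helper to remove any of the four gear mesh components whose matching boolean is off, so each instance keeps only the selected gears.
; On BeginPlay it sets the RotatingMovement component's yaw rate from RotatingSpeed, negated when IsReverse is set.
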(event EventBeginPlay
  (Variables|/Script/Engine.RotatingMovementComponent|SetRotationRate (Variables|Default|GetRotatingMovement) (Math|Rotator|MakeRotator 0.0 0.0 (* (Variables|Default|GetRotatingSpeed) (Math|Float|SelectFloat -1.0 1.0 (Variables|Default|GetIsReverse))))))

(fn ConstructionScript
  (CallFunction|DestroyGear (Variables|Default|GetGear01) (Variables|Default|GetGearMesh01))
  (CallFunction|DestroyGear (Variables|Default|GetGear02) (Variables|Default|GetGearMesh02))
  (CallFunction|DestroyGear (Variables|Default|GetGear03) (Variables|Default|GetGearMesh03))
  (CallFunction|DestroyGear (Variables|Default|GetGear04) (Variables|Default|GetGearMesh04)))

(fn DestroyGear
  (params (Condition :type Boolean) (self2 :type Actor%20Component%20Object%20Reference))
  (if (not Condition)
    (Components|DestroyComponent self2)))