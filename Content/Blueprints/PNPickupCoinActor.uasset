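; Coin pickup actor that adds one coin to the player pawn that touches it.
; A timeline spins the coin's yaw from BeginPlay, while a half-second timer opens a gate so the coin cannot be collected immediately on spawn.
; Once the gate is open, a trigger box overlap with PNPlayerPawn awards the coin, destroys the actor and plays the pickup particle and sound.
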(event OnComponentBeginOverlap(BoxTrigger)
  (params (OverlappedComponent :type Primitive%20Component%20Object%20Reference) (OtherActor :type Actor%20Object%20Reference) (OtherComp :type Primitive%20Component%20Object%20Reference) (OtherBodyIndex :type Integer) (bFromSweep :type Boolean) (SweepResult :type Hit%20Result%20Structure%20%28by%20ref%29))
  (Utilities|FlowControl|Gate true
    (:Exit
      (bind _aspnplayer_pawn (Utilities|Casting|CastToPNPlayerPawn OtherActor))
      (Utilities|FlowControl|Sequence
        (:then_0
          (Default|AddCoin _aspnplayer_pawn 1)
          (Actor|DestroyActor))
        (:then_1
          (Effects|SpawnEmitteratLocation "/Game/Particles/PS_Pickup_Coin.PS_Pickup_Coin" (Transformation|GetActorLocation))
          (Audio|PlaySoundatLocation "/Game/Audio/obj_coin_get_Cue.obj_coin_get_Cue" (Transformation|GetActorLocation) "0, 0, 0" 1.0 1.0 0.0 0 0 0))))))

(event Custom|EnablePickup
  (Utilities|FlowControl|Gate true) ; enters at Open
)

(event EventBeginPlay
  (Utilities|Time|SetTimerbyFunctionName 0 "EnablePickup" 0.5)
  (bind _coinyaw (Timeline|CoinRotationTimeline Play)
    (:Update
      (Transformation|SetActorRelativeRotation (Math|Rotator|MakeRotator 0.0 0.0 _coinyaw)))))

(fn ConstructionScript)