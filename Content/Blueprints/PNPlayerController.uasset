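; PNPlayerController is a player controller that drives camera look and camera-relative pawn movement through a custom PNPlayerCameraManager.
; It caches the camera manager on BeginPlay, feeds scaled look axes into its yaw and pitch, and moves the pawn along the camera's forward and right vectors.
; When notified of obtaining a scroll, it disables camera control, turns the view relative to the pawn's facing, then zooms via FOV after a short delay.
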(event Custom|NotifyObtainedScroll
  (bind _mycameramanager (Variables|Default|GetMyCameraManager))
  (Variables|/Game/Blueprints/PNPlayerCameraManager.PNPlayerCameraManager_C|SetIsEnableControl _mycameramanager false)
  (Variables|/Game/Blueprints/PNPlayerCameraManager.PNPlayerCameraManager_C|SetDesiredRotation _mycameramanager (Math|Rotator|MakeRotator 0.0 2e+01 (- (.Yaw (Math|Rotator|BreakRotator (Transformation|GetActorRotation (Pawn|GetControlledPawn)))) 0.0)))
  (Utilities|FlowControl|Delay 1.0)
  (Variables|/Game/Blueprints/PNPlayerCameraManager.PNPlayerCameraManager_C|SetDesiredFOV _mycameramanager 3e+01))

(event EventBeginPlay
  (bind _aspnplayer_camera_manager (Utilities|Casting|CastToPNPlayerCameraManager (Variables|Default|GetPlayerCameraManager)))
  (Variables|Default|SetMyCameraManager _aspnplayer_camera_manager))

(event EventTick
  (params (DeltaSeconds :type Float%20%28single-precision%29)))

(event Input|AxisEvents|InputAxisLookRight
  (params (AxisValue :type Float%20%28single-precision%29))
  (Default|AddYawInput (Variables|Default|GetMyCameraManager) (* AxisValue 2.5)))

(event Input|AxisEvents|InputAxisLookUp
  (params (AxisValue :type Float%20%28single-precision%29))
  (Default|AddPitchInput (Variables|Default|GetMyCameraManager) (* AxisValue 1.75)))

(event Input|AxisEvents|InputAxisMoveForward
  (params (AxisValue :type Float%20%28single-precision%29))
  (Pawn|Input|AddMovementInput (Pawn|GetControlledPawn) (Default|GetCameraForwardVector (Variables|Default|GetMyCameraManager)) AxisValue false))

(event Input|AxisEvents|InputAxisMoveRight
  (params (AxisValue :type Float%20%28single-precision%29))
  (Pawn|Input|AddMovementInput (Pawn|GetControlledPawn) (Default|GetCameraRightVector (Variables|Default|GetMyCameraManager)) AxisValue false))

(fn ConstructionScript)

(fn GetPNPlayerCameraManager
  (return (Variables|Default|GetMyCameraManager)))