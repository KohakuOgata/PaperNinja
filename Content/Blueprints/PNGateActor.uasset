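; PNGateActor is a gate Actor with two inner door meshes that slide open and closed, with sound effects.
; Open and Close events play or reverse a timeline whose Left vector moves one door, with the other mirrored on Y.
; Timeline event tracks check playback direction so opening and close-end sounds fire only in their direction.
; PlaySE sets an "SE Type" parameter on the Speaker audio component before playing it.
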(event Custom|Open
  (bind (_direction _left) (Timeline|GateTimeline Play)
    (:Update
      (Transformation|SetRelativeLocation (Variables|Default|GetInside%20Left%20Mesh) _left false false)
      (Transformation|SetRelativeLocation (Variables|Default|GetInside%20Right%20Mesh) (* _left "1.000000,-1.000000,1.000000") false false))
    (:Opening
      (if (Utilities|Enum|Equal(Enum) _direction "Forward")
        (CallFunction|PlaySE)))
    (:CloseEnd
      (if (Utilities|Enum|Equal(Enum) _direction "Backward")
        (CallFunction|PlaySE 2)))))

(event Custom|Close
  (CallFunction|PlaySE 1)
  (bind (_direction _left) (Timeline|GateTimeline Reverse)
    (:Update
      (Transformation|SetRelativeLocation (Variables|Default|GetInside%20Left%20Mesh) _left false false)
      (Transformation|SetRelativeLocation (Variables|Default|GetInside%20Right%20Mesh) (* _left "1.000000,-1.000000,1.000000") false false))
    (:Opening
      (if (Utilities|Enum|Equal(Enum) _direction "Forward")
        (CallFunction|PlaySE)))
    (:CloseEnd
      (if (Utilities|Enum|Equal(Enum) _direction "Backward")
        (CallFunction|PlaySE 2)))))

(event EventBeginPlay)

(event Collision|EventActorBeginOverlap
  (params (OtherActor :type Actor%20Object%20Reference)))

(event EventTick
  (params (DeltaSeconds :type Float%20%28single-precision%29)))

(fn ConstructionScript)

(fn PlaySE
  (params (SEType :type Integer))
  (bind _speaker (Variables|Default|GetSpeaker))
  (Effects|Components|ParticleSystem|SetIntParameter _speaker "SE Type" SEType)
  (Audio|Components|Audio|Play _speaker 0.0))